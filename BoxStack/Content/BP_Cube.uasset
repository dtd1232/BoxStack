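; BP_Cube is a cube actor that moves toward a target location until key 1 makes it fall.
; Tick adds a fixed, frame-rate-dependent local offset along the normalized direction to TargetLocation, with Speed wired into Normalize's Tolerance.
; Key 1 sets IsFalling, halting that movement, and plays a timeline that cumulatively adds FallProgress to Z.
; The check stopping the timeline at TargetZ is unconnected and never runs.
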(event `Key|One`
  (params (Key :type "Key Structure"))
  ;[1 1 1] 낙하
  (:`Pressed`
    (set `self.IsFalling` true)
    (bind (_direction _fallprogress) (`Timeline|FallTimeLine` :!via `PlayFromStart`)
      (:`Update`
        (`self.K2_SetActorLocation` (`KismetMathLibrary.MakeVector` (.x (`self.K2_GetActorLocation`)) (.y (`self.K2_GetActorLocation`)) (+ (.z (`self.K2_GetActorLocation`)) _fallprogress)))))))

(event `self.ReceiveTick`
  (params (DeltaSeconds :type "Float (single-precision)"))
  ;[1 1 1] 수평 이동
  (if (not (`self.IsFalling`))
    (`self.K2_AddActorLocalOffset` (* (`KismetMathLibrary.Normal` (- (`self.TargetLocation`) (`self.K2_GetActorLocation`)) (`self.Speed`)) (10.0 10.0 10.0)))))

(fn `UserConstructionScript`)